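; MaterialSphere_Bp is a pellet-folder Blueprint that drives the on-screen score display as pellets are eaten.
; It handles EatPellet events, one per score value up to twenty, each removing the previous score widget and adding a separate widget class for the new value.
; The first event clears any existing Score0 widgets found by class search.
; The Win event opens the WinScreen level.
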(event `self.EatPellet.Score1`
  (bind _foundwidgets (`WidgetBlueprintLibrary.GetAllWidgetsOfClass` "/Game/BluprintClasses/ScoreDisplay/score/Score0.Score0_C"))
  (`Widget.RemoveFromParent` _foundwidgets)
  (bind _returnvalue (`|CreateWidget` "/Game/BluprintClasses/ScoreDisplay/score/Score1.Score1_C"))
  (`UserWidget.AddToViewport` _returnvalue 0))

(event `self.EatPellet.Score2`
  (`Widget.RemoveFromParent` (stale `self.EatPellet.Score1` _returnvalue))
  (bind _returnvalue (`|CreateWidget` "/Game/BluprintClasses/ScoreDisplay/score/Score2.Score2_C"))
  (`UserWidget.AddToViewport` _returnvalue 0))

(event `self.EatPellet.Score3`
  (`Widget.RemoveFromParent` (stale `self.EatPellet.Score2` _returnvalue))
  (bind _returnvalue (`|CreateWidget` "/Game/BluprintClasses/ScoreDisplay/score/Score3.Score3_C"))
  (`UserWidget.AddToViewport` _returnvalue 0))

(event `self.EatPellet.Score4`
  (`Widget.RemoveFromParent` (stale `self.EatPellet.Score3` _returnvalue))
  (bind _returnvalue (`|CreateWidget` "/Game/BluprintClasses/ScoreDisplay/score/Score4.Score4_C"))
  (`UserWidget.AddToViewport` _returnvalue 0))

(event `self.EatPellet.Score5`
  (`Widget.RemoveFromParent` (stale `self.EatPellet.Score4` _returnvalue))
  (bind _returnvalue (`|CreateWidget` "/Game/BluprintClasses/ScoreDisplay/score/Score5.Score5_C"))
  (`UserWidget.AddToViewport` _returnvalue 0))

(event `self.EatPellet.Score6`
  (`Widget.RemoveFromParent` (stale `self.EatPellet.Score5` _returnvalue))
  (bind _returnvalue (`|CreateWidget` "/Game/BluprintClasses/ScoreDisplay/score/Score6.Score6_C"))
  (`UserWidget.AddToViewport` _returnvalue 0))

(event `self.EatPellet.Score7`
  (`Widget.RemoveFromParent` (stale `self.EatPellet.Score6` _returnvalue))
  (bind _returnvalue (`|CreateWidget` "/Game/BluprintClasses/ScoreDisplay/score/Score7.Score7_C"))
  (`UserWidget.AddToViewport` _returnvalue 0))

(event `self.EatPellet.Score8`
  (`Widget.RemoveFromParent` (stale `self.EatPellet.Score7` _returnvalue))
  (bind _returnvalue (`|CreateWidget` "/Game/BluprintClasses/ScoreDisplay/score/Score8.Score8_C"))
  (`UserWidget.AddToViewport` _returnvalue 0))

(event `self.EatPellet.Score9`
  (`Widget.RemoveFromParent` (stale `self.EatPellet.Score8` _returnvalue))
  (bind _returnvalue (`|CreateWidget` "/Game/BluprintClasses/ScoreDisplay/score/Score9.Score9_C"))
  (`UserWidget.AddToViewport` _returnvalue 0))

(event `self.EatPellet.Score10`
  (`Widget.RemoveFromParent` (stale `self.EatPellet.Score9` _returnvalue))
  (bind _returnvalue (`|CreateWidget` "/Game/BluprintClasses/ScoreDisplay/score/Score10.Score10_C"))
  (`UserWidget.AddToViewport` _returnvalue 0))

(event `self.EatPellet.Score11`
  (`Widget.RemoveFromParent` (stale `self.EatPellet.Score10` _returnvalue))
  (bind _returnvalue (`|CreateWidget` "/Game/BluprintClasses/ScoreDisplay/score/Score11.Score11_C"))
  (`UserWidget.AddToViewport` _returnvalue 0))

(event `self.EatPellet.Score12`
  (`Widget.RemoveFromParent` (stale `self.EatPellet.Score11` _returnvalue))
  (bind _returnvalue (`|CreateWidget` "/Game/BluprintClasses/ScoreDisplay/score/Score12.Score12_C"))
  (`UserWidget.AddToViewport` _returnvalue 0))

(event `self.EatPellet.Score13`
  (`Widget.RemoveFromParent` (stale `self.EatPellet.Score12` _returnvalue))
  (bind _returnvalue (`|CreateWidget` "/Game/BluprintClasses/ScoreDisplay/score/Score13.Score13_C"))
  (`UserWidget.AddToViewport` _returnvalue 0))

(event `self.EatPellet.Score14`
  (`Widget.RemoveFromParent` (stale `self.EatPellet.Score13` _returnvalue))
  (bind _returnvalue (`|CreateWidget` "/Game/BluprintClasses/ScoreDisplay/score/Score14.Score14_C"))
  (`UserWidget.AddToViewport` _returnvalue 0))

(event `self.EatPellet.Score15`
  (`Widget.RemoveFromParent` (stale `self.EatPellet.Score14` _returnvalue))
  (bind _returnvalue (`|CreateWidget` "/Game/BluprintClasses/ScoreDisplay/score/Score15.Score15_C"))
  (`UserWidget.AddToViewport` _returnvalue 0))

(event `self.EatPellet.Score16`
  (`Widget.RemoveFromParent` (stale `self.EatPellet.Score15` _returnvalue))
  (bind _returnvalue (`|CreateWidget` "/Game/BluprintClasses/ScoreDisplay/score/Score16.Score16_C"))
  (`UserWidget.AddToViewport` _returnvalue 0))

(event `self.EatPellet.Score17`
  (`Widget.RemoveFromParent` (stale `self.EatPellet.Score16` _returnvalue))
  (bind _returnvalue (`|CreateWidget` "/Game/BluprintClasses/ScoreDisplay/score/Score17.Score17_C"))
  (`UserWidget.AddToViewport` _returnvalue 0))

(event `self.EatPellet.Score18`
  (`Widget.RemoveFromParent` (stale `self.EatPellet.Score17` _returnvalue))
  (bind _returnvalue (`|CreateWidget` "/Game/BluprintClasses/ScoreDisplay/score/Score18.Score18_C"))
  (`UserWidget.AddToViewport` _returnvalue 0))

(event `self.EatPellet.Score19`
  (`Widget.RemoveFromParent` (stale `self.EatPellet.Score18` _returnvalue))
  (bind _returnvalue (`|CreateWidget` "/Game/BluprintClasses/ScoreDisplay/score/Score19.Score19_C"))
  (`UserWidget.AddToViewport` _returnvalue 0))

(event `self.EatPellet.Score20`
  (`Widget.RemoveFromParent` (stale `self.EatPellet.Score19` _returnvalue))
  (bind _returnvalue (`|CreateWidget` "/Game/BluprintClasses/ScoreDisplay/score/Score20.Score20_C"))
  (`UserWidget.AddToViewport` _returnvalue 0))

(event `self.EatPellet.Win`
  (`GameplayStatics.OpenLevel` "WinScreen"))

(fn `UserConstructionScript`)